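; BaseWeaponBP is a base weapon Blueprint that attaches its first- and third-person gun meshes to the owning character.
; The construction script casts the owner to BaseCharacterBP and attaches each mesh to the WeaponPoint socket on the matching character mesh.
; Firing, charging, reload and animation events are empty stubs, and BeginPlay only prints the owner's name.
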(event Custom|PlayShootingAnimation)

(event Custom|PlayChargingAnimation)

(event Custom|OnEndCharging)

(event Custom|OnShotFired)

(event Custom|PlayReloadAnimation)

(event Custom|FireHeld)

(event Custom|FireReleased)

(event Custom|OnStopReloading)

(event Custom|OnStartFiring)

(event Custom|OnStartReload)

(event Custom|OnStartCharging)

(event Custom|OnEndFiring)

(event EventBeginPlay
  (Development|PrintString (Utilities|GetDisplayName (Components|GetOwner))))

(fn ConstructionScript
  (bind _asbase_character_bp (Utilities|Casting|CastToBaseCharacterBP (Components|GetOwner)))
  (Utilities|FlowControl|Sequence
    (:then_0
      (Transformation|AttachComponentToComponent (Variables|Default|GetGunMeshTP) (Variables|/Script/Engine.Character|GetMesh _asbase_character_bp) "WeaponPoint" "KeepRelative" "KeepRelative" "KeepRelative" true))
    (:then_1
      (Transformation|AttachComponentToComponent (Variables|Default|GetGunMeshFP) (Variables|/Game/Blueprints/BaseCharacterBP.BaseCharacterBP_C|GetFirstPersonMesh _asbase_character_bp) "WeaponPoint" "KeepRelative" "KeepRelative" "KeepRelative" true))))